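; BP_WaterPlane is a water hazard that reacts when a BP_CustomTPS actor touches it.
; A Box begin overlap casts the other actor, waits half a second, then calls TPBack and prints a debug message.
; A second sequence branch calls WaterTouched without waiting for that delay.
; The Plane end-overlap event is empty, and a disconnected copy of the overlap logic never runs.
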(event OnComponentEndOverlap(Plane)
  (params (OverlappedComponent :type Primitive%20Component%20Object%20Reference) (OtherActor :type Actor%20Object%20Reference) (OtherComp :type Primitive%20Component%20Object%20Reference) (OtherBodyIndex :type Integer)))

(event OnComponentBeginOverlap(Box)
  (params (OverlappedComponent :type Primitive%20Component%20Object%20Reference) (OtherActor :type Actor%20Object%20Reference) (OtherComp :type Primitive%20Component%20Object%20Reference) (OtherBodyIndex :type Integer) (bFromSweep :type Boolean) (SweepResult :type Hit%20Result%20Structure%20%28by%20ref%29))
  (Utilities|FlowControl|Sequence
    (:then_0
      (bind _asbp_custom_tps (Utilities|Casting|CastToBP_CustomTPS OtherActor))
      (Utilities|FlowControl|Delay 0.5)
      (Default|TPBack _asbp_custom_tps)
      (Development|PrintText "Water Touched"))
    (:then_1
      (Default|WaterTouched _asbp_custom_tps))))

(fn ConstructionScript)